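; BP_Weapon is a weapon actor that reports hits from its Box collider to the owning character's Gameplay Ability System.
; InitWeapon stores the character and attaches the weapon to its mesh at the S_Weapon socket, and ToggleWeaponCollision switches the box collision on or off.
; Box overlaps with other actors send an IntersectionWithWeapon gameplay event to the character, passing the overlapped actor as target.
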(event OnComponentBeginOverlap(Box)
  (params (OverlappedComponent :type Primitive%20Component%20Object%20Reference) (OtherActor :type Actor%20Object%20Reference) (OtherComp :type Primitive%20Component%20Object%20Reference) (OtherBodyIndex :type Integer) (bFromSweep :type Boolean) (SweepResult :type Hit%20Result%20Structure%20%28by%20ref%29))
  (if (and (!= OtherActor self) (!= OtherActor (Variables|Default|GetCharacter)))
    (Ability|SendGameplayEventtoActor (Variables|Default|GetCharacter) "(TagName=\"Ability.Execution.IntersectionWithWeapon\")" (Utilities|Struct|MakeGameplayEventData "(TagName=\"Ability.Execution.IntersectionWithWeapon\")" (Variables|Default|GetCharacter) OtherActor))))

(event Custom|ToggleWeaponCollision
  (params (bEnabled :type Boolean))
  (Collision|SetCollisionEnabled (Variables|Default|GetBox) (select bEnabled "QueryAndPhysics" "NoCollision")))

(event Custom|InitWeapon
  (params (Character :type BP%20Third%20Person%20Character%20Object%20Reference))
  (bind _output_get (Variables|Default|SetCharacter Character))
  (Transformation|AttachComponentToComponent (Variables|/Script/Engine.Character|GetMesh _output_get) "S_Weapon" "SnapToTarget" "SnapToTarget" "SnapToTarget" true))

(event EventBeginPlay)

(event Collision|EventActorBeginOverlap
  (params (OtherActor :type Actor%20Object%20Reference)))

(event EventTick
  (params (DeltaSeconds :type Float%20%28single-precision%29)))

(fn ConstructionScript)