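; BP_Fence is a breakable fence actor that falls apart when something hits it.
; The construction script gathers seven cube components into a Planks array.
; The first hit on the Box component disables that box's collision, then turns on physics and gravity for every plank and applies a fixed-strength impulse along the hit normal.
; A DoOnce keeps the break from repeating.
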(event OnComponentHit(Box)
  (params (HitComponent :type Primitive%20Component%20Object%20Reference) (OtherActor :type Actor%20Object%20Reference) (OtherComp :type Primitive%20Component%20Object%20Reference) (NormalImpulse :type Vector :default "0, 0, 0") (Hit :type Hit%20Result%20Structure%20%28by%20ref%29))
  (if true
    (Utilities|FlowControl|DoOnce false
      (:Completed
        (Collision|SetCollisionEnabled (Variables|Default|GetBox) "NoCollision")
        (for _array_element (Variables|Default|GetPlanks)
          (Physics|SetSimulatePhysics _array_element true)
          (Physics|SetEnableGravity _array_element true)
          (Physics|AddImpulse _array_element (* (Math|Vector|Normalize (.Normal (Collision|BreakHitResult Hit))) "1000.000000,1000.000000,1000.000000") "None" false))))))

(event EventBeginPlay)

(event Collision|EventActorBeginOverlap
  (params (OtherActor :type Actor%20Object%20Reference)))

(event EventTick
  (params (DeltaSeconds :type Float%20%28single-precision%29)))

(fn ConstructionScript
  (Variables|Default|SetPlanks (Utilities|Array|MakeArray (Variables|Default|GetCube) (Variables|Default|GetCube1) (Variables|Default|GetCube2) (Variables|Default|GetCube3) (Variables|Default|GetCube4) (Variables|Default|GetCube5) (Variables|Default|GetCube6))))