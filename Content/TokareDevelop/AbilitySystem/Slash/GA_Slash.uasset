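; Gameplay ability for a three-step grounded slash combo, choosing the attack montage from the GE_Slash_Stack count.
; Movement is disabled at start; gameplay events mark the active phase, whose end restores movement, advances or resets the timed stack, and lets confirm end the ability early.
; Weapon-intersection events collect unique enemies, but hit and trace handlers only print, applying no damage.
; Ending mid-active phase still finishes that phase.
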(event Custom|FinishActivePhase
  (bind _character (Variables|Default|GetCharacter))
  (bind _returnvalue (Ability|GetAbilitySystemComponent _character))
  (if (< (GameplayEffects|GetGameplayEffectCount (Ability|GetAbilitySystemComponent (Ability|GetAvatarActorfromActorInfo)) "/Game/TokareDevelop/AbilitySystem/Slash/GE_Slash_Stack.GE_Slash_Stack_C" 0 true) 2)
    (CallFunction|UpdateCurrentStacks 1)
    (else
      (GameplayEffects|RemoveActiveEffectswithGrantedTags _returnvalue "(GameplayTags=((TagName=\"Ability.Slash.Stack\")))")))
  (Variables|Default|SetbActivePhaseFinished true)
  (GameplayEffects|RemoveActiveGameplayEffect _returnvalue (Variables|Default|GetHandle_ActivePhase) -1)
  (GameplayEffects|RemoveActiveGameplayEffect (Ability|GetAbilitySystemComponent (Ability|GetAvatarActorfromActorInfo)) (Variables|Default|GetHandle_DisableMovement) -1))

(event Custom|UpdateCurrentStacks
  (params (StackCount :type Integer))
  (bind _character (Variables|Default|GetCharacter))
  (bind _returnvalue (Ability|GetAbilitySystemComponent _character))
  (bind _returnvalue_2 (Ability|GameplayEffect|AssignTagSetbyCallerMagnitude (GameplayEffects|MakeOutgoingSpec _returnvalue "/Game/TokareDevelop/AbilitySystem/Slash/GE_Slash_Stack.GE_Slash_Stack_C" 1.0 (GameplayEffects|MakeEffectContext _returnvalue)) "(TagName=\"Effect.Data.Duration\")" 2.0))
  (bind _returnvalue_3 (Class|AbilitySystemBlueprintLibrary|SetStackCount _returnvalue_2 StackCount))
  (GameplayEffects|ApplyGameplayEffectSpecToSelf _returnvalue _returnvalue_3))

(event Custom|OnActivePhaseStarted
  (bind _returnvalue (Ability|ApplyGameplayEffectToOwner "/Game/TokareDevelop/AbilitySystem/GE_AbilityActivePhase.GE_AbilityActivePhase_C"))
  (Variables|Default|SetHandle_ActivePhase _returnvalue)
  (Variables|Default|SetbActivePhaseStarted true))

(event Custom|OnActivePhaseFinished
  (CallFunction|FinishActivePhase)
  (|WaitConfirmCancel
    (:OnConfirm
      (Ability|EndAbility))))

(event Custom|OnTargetReached
  (params (Target :type Actor%20Object%20Reference))
  (bind _asbp_enemy (Utilities|Casting|CastToBP_Enemy Target))
  (bind _returnvalue (Utilities|Array|AddUnique (Variables|Default|GetAffectedEnemies) _asbp_enemy))
  (if (!= _returnvalue -1)
    (Development|PrintString (Utilities|GetDisplayName Target) true true "(R=1.000000,G=0.450211,B=0.000000,A=1.000000)" 3.0)))

(event Custom|OnPerformTrace
  (Development|PrintString "TRACE" true true "(R=1.000000,G=0.036947,B=0.000000,A=1.000000)" 3.0))

(event Ability|EventActivateAbility
  (bind _asbp_third_person_character (Utilities|Casting|CastToBP_ThirdPersonCharacter (Ability|GetAvatarActorfromActorInfo))
    (:then
      (Variables|Default|SetCharacter _asbp_third_person_character)
      (if (not (AI|Components|NavMovement|IsFalling (Variables|/Script/Engine.Character|GetCharacterMovement (Variables|Default|GetCharacter))))
        (|PlayMontageandWaitProxy "None" (Utilities|Select :Index (GameplayEffects|GetGameplayEffectCount (Ability|GetAbilitySystemComponent (Variables|Default|GetCharacter)) "/Game/TokareDevelop/AbilitySystem/Slash/GE_Slash_Stack.GE_Slash_Stack_C" 0 true) :Option%200 "/Game/TokareDevelop/Characters/Paladin/Animations/Montages/AM_Paladin_Attack_1.AM_Paladin_Attack_1" :Option%201 "/Game/TokareDevelop/Characters/Paladin/Animations/Montages/AM_Paladin_Attack_2.AM_Paladin_Attack_2" :Option%202 "/Game/TokareDevelop/Characters/Paladin/Animations/Montages/AM_Paladin_Attack_3.AM_Paladin_Attack_3") 1.0 "None" true 1.0 0.0
          (:then
            (bind _returnvalue (Ability|ApplyGameplayEffectToOwner "/Game/TokareDevelop/AbilitySystem/GE_DisableMovement.GE_DisableMovement_C"))
            (Variables|Default|SetHandle_DisableMovement _returnvalue)
            (CallFunction|UpdateCurrentStacks)
            (Variables|Default|SetbActivePhaseStarted false)
            (Variables|Default|SetbActivePhaseFinished false)
            (Utilities|Array|Clear (Variables|Default|GetAffectedEnemies))
            (Ability|Tasks|WaitGameplayEvent "(TagName=\"Ability.State.ActivePhaseStarted\")" 0
              (:then
                (Ability|Tasks|WaitGameplayEvent "(TagName=\"Ability.State.ActivePhaseFinished\")" 0
                  (:then
                    (bind _payload (Ability|Tasks|WaitGameplayEvent "(TagName=\"Ability.Execution.IntersectionWithWeapon\")" 0)
                      (:then
                        (Ability|Tasks|WaitGameplayEvent "(TagName=\"Ability.Execution.PerformTrace\")" 0
                          (:EventReceived
                            (CallFunction|OnPerformTrace))))
                      (:EventReceived
                        (CallFunction|OnTargetReached (.Target (Utilities|Struct|BreakGameplayEventData _payload))))))
                  (:EventReceived
                    (CallFunction|OnActivePhaseFinished))))
              (:EventReceived
                (CallFunction|OnActivePhaseStarted))))
          (:OnCompleted
            (Ability|EndAbility :!label _label))
          (:OnBlendOut
            (goto _label))
          (:OnInterrupted
            (goto _label))
          (:OnCancelled
            (goto _label)))
        (else
          (Ability|EndAbility))))
    (:CastFailed
      (Ability|EndAbility))))

(event Ability|EventOnEndAbility
  (params (bWasCancelled :type Boolean))
  (bind _character (Variables|Default|GetCharacter))
  (bind _returnvalue (Ability|GetAbilitySystemComponent _character))
  (GameplayEffects|RemoveActiveGameplayEffect _returnvalue (Variables|Default|GetHandle_ActivePhase) -1)
  (GameplayEffects|RemoveActiveGameplayEffect _returnvalue (Variables|Default|GetHandle_DisableMovement) -1)
  (if (and (Variables|Default|GetbActivePhaseStarted) (not (Variables|Default|GetbActivePhaseFinished)))
    (CallFunction|FinishActivePhase)))