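; Dash gameplay ability that instantly moves the avatar up to 400 units along the camera's horizontal forward, turning it to the camera's yaw.
; A Visibility line trace shortens the swept move at obstacles; the flattened direction is not renormalized, so camera pitch reduces range.
; It then self-applies GE_Impulse with a set-by-caller duration.
; CommitAbility runs only after the move and effect, immediately before the ability ends.
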(event Ability|EventActivateAbility
  (bind _returnvalue (Ability|GetAvatarActorfromActorInfo))
  (bind _returnvalue_2 (Ability|GetAvatarActorfromActorInfo))
  (bind _returnvalue_3 (Ability|GetAbilitySystemComponent _returnvalue))
  (bind _returnvalue_4 (Actor|GetComponentbyClass _returnvalue_2 "/Script/Engine.CameraComponent"))
  (bind _returnvalue_5 (Transformation|GetActorLocation _returnvalue_2))
  (bind _returnvalue_6 (Transformation|GetActorRotation _returnvalue_2))
  (bind (_roll _pitch) (Math|Rotator|BreakRotator _returnvalue_6))
  (bind (_outhit _returnvalue_7) (Collision|LineTraceByChannel _returnvalue_5 (+ _returnvalue_5 (* (Math|Conversions|ToVector2D(Vector) (Math|Vector|GetForwardVector _returnvalue_4)) 4e+02)) "TraceTypeQuery1" false 0 "None"))
  (Transformation|SetActorLocationAndRotation (Ability|GetAvatarActorfromActorInfo) (select (not _returnvalue_7) (.TraceEnd (Collision|BreakHitResult _outhit)) (.Location (Collision|BreakHitResult _outhit))) (Math|Rotator|MakeRotator _roll _pitch (.Yaw (Math|Rotator|BreakRotator (Transformation|GetWorldRotation _returnvalue_4)))) true)
  (bind _returnvalue_8 (Ability|GameplayEffect|AssignTagSetbyCallerMagnitude (GameplayEffects|MakeOutgoingSpec _returnvalue_3 "/Game/TokareDevelop/AbilitySystem/GE_Impulse.GE_Impulse_C" 1.0 (GameplayEffects|MakeEffectContext _returnvalue_3)) "(TagName=\"Effect.Data.Duration\")" 0.5))
  (GameplayEffects|ApplyGameplayEffectSpecToSelf _returnvalue_3 _returnvalue_8)
  (Ability|CommitAbility)
  (Ability|EndAbility))

(event Ability|EventOnEndAbility
  (params (bWasCancelled :type Boolean)))